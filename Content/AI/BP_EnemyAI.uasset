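; Enemy AI actor that detects the player character and deals damage through mesh contact.
; PawnSensing sightings of BP_GEPCharacter set the HasSeenPlayer blackboard key on the AI controller to true.
; Any overlap on the mesh applies fixed damage to the player, without checking the overlapping actor.
; On player death, ResetAI disables sensing updates but also sets HasSeenPlayer to true rather than clearing it.
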(event `self.ReceiveBeginPlay`
  (bind _asbp_gepcharacter (cast `/Game/BP_GEPCharacter` (`GameplayStatics.GetPlayerCharacter` 0)))
  (add `/Game/BP_GEPCharacter.PlayerDied` _asbp_gepcharacter (delegate `ResetAI`)))

(event `ResetAI`
  (`PawnSensingComponent.SetSensingUpdatesEnabled` (`self.PawnSensing`) false)
  (`BlackboardComponent.SetValueAsBool` (`AIBlueprintHelperLibrary.GetBlackboard` (`AIBlueprintHelperLibrary.GetAIController` self)) "HasSeenPlayer" true))

(event `self.ReceiveActorBeginOverlap`
  (params (OtherActor :type "Actor Object Reference")))

(event `self.PawnSensing.OnSeePawn`
  (params (Pawn :type "Pawn Object Reference"))
  (cast `/Game/BP_GEPCharacter` Pawn)
  (`BlackboardComponent.SetValueAsBool` (`AIBlueprintHelperLibrary.GetBlackboard` (`AIBlueprintHelperLibrary.GetAIController` self)) "HasSeenPlayer" true))

(event `self.Mesh.OnComponentBeginOverlap`
  (params (OverlappedComponent :type "PrimitiveComponent Object Reference") (OtherActor :type "Actor Object Reference") (OtherComp :type "PrimitiveComponent Object Reference") (OtherBodyIndex :type Integer) (bFromSweep :type Boolean) (SweepResult :type "HitResult Structure (by ref)"))
  (bind _asbp_gepcharacter (cast `/Game/BP_GEPCharacter` (`GameplayStatics.GetPlayerCharacter` 0)))
  (`GameplayStatics.ApplyDamage` _asbp_gepcharacter 10.0 null self))

(fn `UserConstructionScript`)